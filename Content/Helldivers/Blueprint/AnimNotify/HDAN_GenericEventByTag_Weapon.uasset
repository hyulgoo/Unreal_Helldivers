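; Anim notify for weapon animations that sends a configurable gameplay event tag to the actor owning the weapon.
; It resolves the target as the owner of the mesh component's owner, so an event fired from a weapon mesh reaches its owning actor.
; The payload carries only the event tag, and the notify displays that tag as its name.
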(fn ReceivedNotify
  (params (MeshComp :type Skeletal%20Mesh%20Component%20Object%20Reference) (Animation :type Anim%20Sequence%20Base%20Object%20Reference) (EventReference :type Anim%20Notify%20Event%20Reference%20Structure%20%28by%20ref%29))
  (bind _eventtag (Variables|Default|GetEventTag))
  (Ability|SendGameplayEventtoActor (Components|GetOwner (Components|GetOwner MeshComp)) _eventtag (Utilities|Struct|MakeGameplayEventData _eventtag))
  (return false))

(fn GetNotifyName
  (return (Utilities|String|ToString(Name) (GameplayTags|GetTagName (Variables|Default|GetEventTag)))))